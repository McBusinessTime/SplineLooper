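; CarMesh is a Blueprint example class in SplineLooper that gives its static mesh a randomized material look.
; The Construction Script creates a dynamic material instance on the mesh's first material slot, then sets random Color, Metallic and Roughness parameters.
; Randomization is unseeded, so the look can change whenever construction reruns.
; The event graph holds only disabled placeholder events, so it adds no runtime logic.
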(event EventBeginPlay)

(event Collision|EventActorBeginOverlap
  (params (OtherActor :type Actor%20Object%20Reference)))

(event EventTick
  (params (DeltaSeconds :type Float%20%28single-precision%29)))

(fn ConstructionScript
  ;[0 0 0] Randomize Color and Shader
  (bind _returnvalue (Rendering|Material|CreateDynamicMaterialInstance (Variables|Default|GetStaticMesh) 0 0 :!class /Script/Engine.PrimitiveComponent))
  (Rendering|Material|SetVectorParameterValue _returnvalue "Color" (Utilities|Struct|MakeLinearColor (Math|Random|RandomFloatinRange 0.0 1.0) (Math|Random|RandomFloatinRange 0.0 1.0) (Math|Random|RandomFloatinRange 0.0 1.0) 1.0) :!class /Script/Engine.MaterialInstanceDynamic)
  (Rendering|Material|SetScalarParameterValue _returnvalue "Metallic" (Math|Random|RandomFloatinRange 0.0 1.0) :!class /Script/Engine.MaterialInstanceDynamic)
  (Rendering|Material|SetScalarParameterValue _returnvalue "Roughness" (Math|Random|RandomFloatinRange 0.0 1.0) :!class /Script/Engine.MaterialInstanceDynamic))